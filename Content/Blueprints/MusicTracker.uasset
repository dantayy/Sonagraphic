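; MusicTracker is an actor that plays a 2D music track on BeginPlay and flags its beats through OnBeat.
; Each Tick samples the track's frequency spectrum at game time, assuming playback matches that clock, and thresholds the normalized lowest band.
; A frame-counted Delay holds OnBeat after each hit, with debug printing on beats.
; Unwired leftover logic records that band's low and high extremes.
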(event EventBeginPlay
  (Audio|PlaySound2D (Variables|Default|GetSOUND)))

(event Collision|EventActorBeginOverlap
  (params (OtherActor :type Actor%20Object%20Reference)))

(event EventTick
  (params (DeltaSeconds :type Float%20%28single-precision%29))
  (bind _outspectrum (Class|SoundVisualizationStatics|CalculateFrequencySpectrum (Variables|Default|GetSOUND) 0 (Utilities|Time|GetGameTimeinSeconds) 0.01 10))
  (bind _output_get (Variables|Default|SetFrequencies _outspectrum))
  (if (> (Math|Float|NormalizetoRange (Utilities|Array|Get(acopy) _output_get) 2e+01 7e+01) 0.7)
    (Variables|Default|SetonBeat true)
    (Development|PrintString (Utilities|String|ToString(Float) (Math|Float|NormalizetoRange (Utilities|Array|Get(acopy) _output_get) 2e+01 7e+01)) true true "(R=1.000000,G=0.000000,B=0.000000,A=1.000000)" 0.1)
    (Variables|Default|Setdelay 20)
    (elif (> (Variables|Default|Getdelay) 0)
      (bind _result (Math|Integer|DecrementInt (Variables|Default|Getdelay)))
      (else
        (Variables|Default|SetonBeat false)))))

(fn ConstructionScript)