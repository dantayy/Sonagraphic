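; Weapon actor with automatic fire and a rhythm-timed special shot gated by a MusicTracker's OnBeat flag, checked every tick.
; Holding the trigger spawns projectiles on a looping timer at RoundsPerSecond.
; On-beat special shots trace past enemies and spawn a short-lived projectile stretched to the impact point, widening with each consecutive hit.
; Off-beat presses jam the special fire briefly and reset the streak.
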(event Custom|PullTrigger
  (Utilities|FlowControl|DoOnce false
    (:Completed
      (CallFunction|Fire)
      (Utilities|Time|SetTimerbyFunctionName 0 "Fire" (/ 1.0 (Variables|Default|GetroundsPerSecond)) true))))

(event Custom|PullSpecialTrigger
  (if (not (Variables|Default|Getjammed))
    (if (Variables|Default|GetcanSpecialFire)
      (CallFunction|SpecialFire)
      (Math|Integer|IncrementInt (Variables|Default|GetconsecutiveOnBeatHits))
      (else
        (Variables|Default|Setjammed true)
        (Variables|Default|SetconsecutiveOnBeatHits 0)
        (Utilities|FlowControl|Delay 2.0)
        (Variables|Default|Setjammed false)))))

(event Custom|SpecialFire
  (bind _projectilespawnpoint (Variables|Default|GetProjectileSpawnPoint))
  (bind _returnvalue (Transformation|GetWorldLocation _projectilespawnpoint))
  (bind _outactors (Actor|GetAllActorsOfClass "/Game/Blueprints/EnemyCharacter.EnemyCharacter_C"))
  (bind (_outhit _returnvalue_2) (Collision|LineTraceByChannel _returnvalue (+ _returnvalue (* (Math|Vector|GetForwardVector _projectilespawnpoint) 9999)) "TraceTypeQuery1" false _outactors "None"))
  (if _returnvalue_2
    (bind _returnvalue_3 (Game|SpawnActorfromClass "/Game/Blueprints/Projectile.Projectile_C" (Transformation|GetWorldTransform _projectilespawnpoint) "Undefined" 0 0))
    (Transformation|SetWorldScale3D (Variables|/Game/Blueprints/Projectile.Projectile_C|GetDefaultSceneRoot _returnvalue_3) (Math|Vector|MakeVector (Math|Vector|VectorLength (- (.ImpactPoint (Collision|BreakHitResult _outhit)) (.TraceStart (Collision|BreakHitResult _outhit)))) (+ (* (Variables|Default|GetconsecutiveOnBeatHits) 0.1) 1.0) 1.0))
    (if true
      (Utilities|FlowControl|Delay 0.1)
      (Actor|DestroyActor _returnvalue_3))))

(event Custom|ReleaseTrigger
  (Utilities|Time|ClearTimerbyFunctionName 0 "Fire")
  (Utilities|FlowControl|DoOnce false) ; enters at Reset
)

(event Custom|Fire
  (Game|SpawnActorfromClass "/Game/Blueprints/Projectile.Projectile_C" (Transformation|GetWorldTransform (Variables|Default|GetProjectileSpawnPoint)) "Undefined" 0 0))

(event EventBeginPlay)

(event EventTick
  (params (DeltaSeconds :type Float%20%28single-precision%29))
  (bind _outactors (Actor|GetAllActorsOfClass "/Game/Blueprints/MusicTracker.MusicTracker_C"))
  (if (Variables|/Game/Blueprints/MusicTracker.MusicTracker_C|GetonBeat (Utilities|Array|Get(acopy) _outactors))
    (Variables|Default|SetcanSpecialFire true)
    (else
      (Variables|Default|SetcanSpecialFire false))))

(fn ConstructionScript)